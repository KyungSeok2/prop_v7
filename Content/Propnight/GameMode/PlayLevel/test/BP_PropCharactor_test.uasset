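; BP_PropCharactor_test is a test prop character that moves as a physics-driven static mesh.
; MoveForward and MoveRight axes apply mass-independent forces to the mesh along control-yaw forward and right vectors.
; Tick rotates the spring arm from input axis values, and BeginPlay attaches a component to the mesh with relative transforms kept.
; Torque-based movement nodes remain in the graph but never run.
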(event `InputAxis|MoveRight`
  (params (AxisValue :type "Float (single-precision)"))
  ;[1 1 1] 코멘트
)

(event `InputAxis|MoveForward`
  (params (AxisValue :type "Float (single-precision)"))
  ;[1 1 1] 코멘트
)

(event `InputAxis|MoveForward` :overrideparent false
  (params (AxisValue :type "Float (single-precision)"))
  (`PrimitiveComponent.AddForce` (`self.Static Mesh`) (* (`KismetMathLibrary.GetForwardVector` (`KismetMathLibrary.MakeRotator` 0.0 0.0 (.yaw (`self.GetControlRotation`)))) (* AxisValue 1500.0)) "None" true))

(event `self.ReceiveTick`
  (params (DeltaSeconds :type "Float (single-precision)"))
  (`SceneComponent.K2_AddRelativeRotation` (`self.SpringArm`) (`KismetMathLibrary.MakeRotator` 0.0 (`self.GetInputAxisKeyValue`) (`self.GetInputAxisKeyValue`)) false false))

(event `InputAxis|MoveRight` :overrideparent false
  (params (AxisValue :type "Float (single-precision)"))
  (`PrimitiveComponent.AddForce` (`self.Static Mesh`) (* (`KismetMathLibrary.GetRightVector` (`KismetMathLibrary.MakeRotator` 0.0 0.0 (.yaw (`self.GetControlRotation`)))) (* AxisValue 1500.0)) "None" true))

(event `self.ReceiveBeginPlay`
  (`self.K2_AttachToComponent` (`self.Static Mesh`) "None" "KeepRelative" "KeepRelative" "KeepRelative"))

(fn `UserConstructionScript`)